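; Test Blueprint for a player-driven chassis (Dipan) with a rotatable base and pitch pivot, controlled through input axes.
; MoveVertical offsets the actor along its forward vector by MoveSpeed, without sweep collision.
; RotateHorizontal yaws the DizuoStaticMesh base and RotateVertical pitches the Scene component, both scaled by RotateSpeed.
; Movement and rotation apply raw per-call axis values without delta-time scaling; BeginPlay, Tick and construction are empty.
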(event `InputAxis|MoveVertical`
  (params (AxisValue :type "Float (single-precision)"))
  (`self.K2_AddActorWorldOffset` (* (`self.GetActorForwardVector`) (* (`self.moveSpeed`) AxisValue))))

(event `InputAxis|RotateHorizontal`
  (params (AxisValue :type "Float (single-precision)"))
  (`SceneComponent.K2_AddLocalRotation` (`self.Dizuo_StaticMesh`) (`KismetMathLibrary.MakeRotator` 0.0 0.0 (* AxisValue (`self.rotateSpeed`))) false false))

(event `InputAxis|RotateVertical`
  (params (AxisValue :type "Float (single-precision)"))
  (`SceneComponent.K2_AddLocalRotation` (`self.Scene`) (`KismetMathLibrary.MakeRotator` 0.0 (* AxisValue (`self.rotateSpeed`))) false false))

(fn `UserConstructionScript`)