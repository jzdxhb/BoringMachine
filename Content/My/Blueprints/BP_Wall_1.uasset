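; BP_Wall_1 is a breakable wall with health, built on a destructible component.
; BeginPlay sets current health to the total, and the TakeDamage function subtracts incoming damage from it.
; Once health drops to zero or below, it passes the hit position and direction to the destructible component as fixed damage and impulse, then marks the wall dead.
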(event `self.ReceiveBeginPlay`
  (set `self.curHealth` (`self.totelHealth`)))

(fn `TakeDamage`
  (params (damage :type "Float (double-precision)") (HitPos :type "Vector Structure") (HitDir :type "Vector Structure"))
  (bind _output_get (set `self.curHealth` (- (`self.curHealth`) damage)))
  (if (<= _output_get 0.0)
    (`DestructibleComponent.ApplyDamage` (`self.DestructibleComponent`) 10.0 HitPos HitDir 1.0)
    (set `self.isDead` true)))

(fn `UserConstructionScript`)