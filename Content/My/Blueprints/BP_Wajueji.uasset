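; Player-drivable tunnel boring machine that moves forward and back, swings its cutting arm within clamped angles and drills through coal walls.
; Axis inputs drive movement and arm while the engine runs, and a timeline ramps drill spin up and down.
; Drill overlaps track BP_Wall_1 actors, which take damage each tick while drilling and trigger particle effects.
; Wall contact damps arm rotation and lerped forward speed, varying with whether the drill runs.
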(event `self.ReceiveTick`
  (params (DeltaSeconds :type "Float (single-precision)"))
  (`|ExecutionSequence`
    (:`then_0`
      (`self.DrillRot`))
    (:`then_1`
      (bind _isinwall (`self.DrillIsInWall`))
      (if _isinwall
        ;[1 1 1] 根据是否在墙里和钻头是否正在工作调整不同的阻尼系数
        (if (`self.drillWork`)
          (set `self.armRotateDamp` (* (`self.armrotateSpeed`) 0.5))
          (set `self.moveSpeedDamp` (* (`self.moveMaxSpeed`) 0.95))
          (set `self.moveSpeedLerpValue` 0.05)
          (else
            (set `self.armRotateDamp` (`self.armrotateSpeed`))
            (set `self.moveSpeedDamp` (`self.moveMaxSpeed`))
            (set `self.moveSpeedLerpValue` 1.0)))
        (else
          (`self.ResetAllDampPrameter`))))
    (:`then_2`
      (`self.SmokeSwitch`))
    (:`then_3`
      (`self.BreakTheWall`))))

(event `InputAxis|MoveVertical`
  (params (AxisValue :type "Float (single-precision)"))
  (`self.BoringMachineMovement` AxisValue))

(event `InputAxis|RotateHorizontal`
  (params (AxisValue :type "Float (single-precision)"))
  (bind (_relativerotation_roll _relativerotation_pitch _relativerotation_yaw) (`KismetMathLibrary.BreakRotator` (`SceneComponent.RelativeRotation` (`self.20180124_zhuanlun_001`))))
  ;[1 1 1] 摇臂上下左右旋转
  (if (`self.engineIsStart`)
    (`SceneComponent.K2_AddWorldRotation` (`self.20180124_zhuanlun_001`) (`KismetMathLibrary.MakeRotator` 0.0 0.0 (* AxisValue (- (`self.armrotateSpeed`) (`self.armRotateDamp`)))) false false)
    (`SceneComponent.K2_SetRelativeRotation` (`self.20180124_zhuanlun_001`) (`KismetMathLibrary.MakeRotator` _relativerotation_roll _relativerotation_pitch (`KismetMathLibrary.ClampAngle` _relativerotation_yaw (`self.drillHorizontalMinAngle`) (`self.drillHorizontalMaxAngle`))) false false)))

(event `InputAxis|RotateVertical`
  (params (AxisValue :type "Float (single-precision)"))
  (bind (_relativerotation_roll _relativerotation_pitch _relativerotation_yaw) (`KismetMathLibrary.BreakRotator` (`SceneComponent.RelativeRotation` (`self.20180124_qianzhilun4`))))
  ;[1 1 1] 摇臂上下左右旋转
  (if (`self.engineIsStart`)
    (`SceneComponent.K2_AddLocalRotation` (`self.20180124_qianzhilun4`) (`KismetMathLibrary.MakeRotator` 0.0 (* AxisValue (- (`self.armrotateSpeed`) (`self.armRotateDamp`)))) false false)
    (`SceneComponent.K2_SetRelativeRotation` (`self.20180124_qianzhilun4`) (`KismetMathLibrary.MakeRotator` _relativerotation_roll (`KismetMathLibrary.ClampAngle` _relativerotation_pitch (`self.drillVerticalMinAngle`) (`self.drillVerticalMaxAngle`)) _relativerotation_yaw) false false)))

(event `InputAction|DrillWork`
  (params (Key :type "Key Structure" :default "AnyKey"))
  ;[1 1 1] 钻头的开关
  (:`Pressed`
    (if (`self.engineIsStart`)
      (bind _output_get (set `self.drillWork` (not (`self.drillWork`))))
      (if _output_get
        (bind (_direction _newtrack_0) (`Timeline|DrillRotateSpeedLine` :!via `PlayFromStart` :!label _label)
          (:`Update`
            (set `self.drillRotateSpeed` _newtrack_0)))
        (else
          (goto _label :!via `ReverseFromEnd`))))))

(event `self.20180123_zhuanlun_001.OnComponentBeginOverlap`
  (params (OverlappedComponent :type "PrimitiveComponent Object Reference") (OtherActor :type "Actor Object Reference") (OtherComp :type "PrimitiveComponent Object Reference") (OtherBodyIndex :type Integer) (bFromSweep :type Boolean) (SweepResult :type "HitResult Structure (by ref)"))
  (bind _asbp_wall_1 (cast `/Game/My/Blueprints/BP_Wall_1` OtherActor))
  (if (not (`/Game/My/Blueprints/BP_Wall_1.isDead` _asbp_wall_1))
    (`KismetArrayLibrary.Array_Add` (`self.wall`) _asbp_wall_1)))

(event `self.20180123_zhuanlun_001.OnComponentEndOverlap`
  (params (OverlappedComponent :type "PrimitiveComponent Object Reference") (OtherActor :type "Actor Object Reference") (OtherComp :type "PrimitiveComponent Object Reference") (OtherBodyIndex :type Integer))
  (bind _asbp_wall_1 (cast `/Game/My/Blueprints/BP_Wall_1` OtherActor))
  (`KismetArrayLibrary.Array_RemoveItem` (`self.wall`) _asbp_wall_1))

(fn `BoringMachineMovement`
  (params (axisValue :type "Float (double-precision)"))
  (if (`self.engineIsStart`)
    (if (>= axisValue 0.0)
      (set `self.curMoveSpeed` (`KismetMathLibrary.Lerp` (`self.curMoveSpeed`) (* axisValue (- (`self.moveMaxSpeed`) (`self.moveSpeedDamp`))) (`self.moveSpeedLerpValue`)))
      (`self.K2_AddActorWorldOffset` (* (`self.GetActorForwardVector`) (`self.curMoveSpeed`)))
      (else
        (set `self.curMoveSpeed` (`KismetMathLibrary.Lerp` (`self.curMoveSpeed`) (* axisValue (`self.moveMaxSpeed`)) 0.01))
        (`self.K2_AddActorWorldOffset` (* (`self.GetActorForwardVector`) (`self.curMoveSpeed`)))))))

(fn `BreakTheWall`
  (bind _returnvalue (`SceneComponent.K2_GetComponentLocation` (`self.Box`)))
  ;[1 1 1] 煤层受到伤害并且破碎
  (if (and (`self.drillWork`) (`self.isInWall`))
    (for _array_element (`self.wall`)
      (`/Game/My/Blueprints/BP_Wall_1.TakeDamage` _array_element 1.0 _returnvalue _returnvalue))))

(fn `DrillIsInWall`
  (returns (isInWall :type Boolean))
  ;[1 1 1] 判断钻头是否在墙里
  (if (<= (`KismetArrayLibrary.Array_Length` (`self.wall`)) 0)
    (bind _output_get (set `self.isInWall` false))
    (return _output_get)
    (else
      (bind _output_get_2 (set `self.isInWall` true))
      (return _output_get_2))))

(fn `DrillRot`
  ;[1 1 1] 钻头旋转逻辑
  (if (`self.engineIsStart`)
    (`SceneComponent.K2_AddLocalRotation` (`self.20180123_zhuanlun_001`) (* (`KismetMathLibrary.MakeRotator` 1.0) (* (`GameplayStatics.GetWorldDeltaSeconds`) (`self.drillRotateSpeed`))) false false)))

(fn `GetPlayerControllerPossess`
  (`self.EnableInput` (`GameplayStatics.GetPlayerController` 0)))

(fn `GiveUpPlayerController`
  (`self.DisableInput` (`GameplayStatics.GetPlayerController` 0)))

(fn `ResetAllDampPrameter`
  (set `self.armRotateDamp` 0.0)
  (set `self.moveSpeedDamp` 0.0)
  (set `self.moveSpeedLerpValue` 0.01))

(fn `SmokeSwitch`
  ;[1 1 1] 钻头火星烟雾特效的开关
  (if (and (`self.isInWall`) (`self.drillWork`))
    (`ActorComponent.Activate` (`self.zuantouParticaleSystem`) false)
    (else
      (`ActorComponent.Deactivate` (`self.zuantouParticaleSystem`)))))

(fn `StartOrStopEngine`
  (set `self.engineIsStart` (not (`self.engineIsStart`))))

(fn `UserConstructionScript`)